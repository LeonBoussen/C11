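; BP_MicCaptureWithEffects is an actor that captures microphone audio and exposes its volume envelope as a value.
; On BeginPlay it activates and starts an AudioCapture component, with short delays before each step.
; The component's envelope event writes the current level to MicOutputNaarVR.
; Tick only stores delta time, used by a disconnected debug print of the envelope.
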(event `self.AudioCapture.OnAudioEnvelopeValue`
  (params (EnvelopeValue :type "Float (single-precision)"))
  ;[1 1 1] volume envelope
  (bind _output_get (set `self.micOutputNaarVR` EnvelopeValue)))

(event `self.ReceiveBeginPlay`
  (`KismetSystemLibrary.Delay` 0.2)
  (`ActorComponent.Activate` (`self.AudioCapture`) false)
  (`KismetSystemLibrary.Delay` 0.2)
  (`SynthComponent.Start` (`self.AudioCapture`)))

(event `self.ReceiveTick`
  (params (DeltaSeconds :type "Float (single-precision)"))
  ;[1 1 1] tick
  (`|ExecutionSequence`
    (:`then_1`
      (set `self.deltaTick` DeltaSeconds))))

(fn `UserConstructionScript`)