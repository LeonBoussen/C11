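; VR player pawn that handles thumbstick movement, physics-driven hands and a flashlight.
; On BeginPlay it sets floor tracking and binds physics-simulated hand models to hand position components through constraints.
; Both left thumbstick axes add movement along the camera's forward vector.
; SwitchFlashlight runs at start and on trigger overlap, but both branches attach the flashlight to the camera and leave FlashlightOnHand unchanged.
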(event `self.ReceiveBeginPlay`
  (`|ExecutionSequence`
    (:`then_0`
      (`HeadMountedDisplayFunctionLibrary.SetTrackingOrigin` "Floor")
      (`self.SimulateHandPhysics`)
      (`self.SwitchFlashlight`))))

(event `InputAxis|MotionControllerThumbLeft_X`
  (params (AxisValue :type "Float (single-precision)"))
  (`self.AddMovementInput` (`SceneComponent.GetForwardVector` (`self.Camera`)) AxisValue))

(event `InputAxis|MotionControllerThumbLeft_Y`
  (params (AxisValue :type "Float (single-precision)"))
  (`self.AddMovementInput` (`SceneComponent.GetForwardVector` (`self.Camera`)) AxisValue))

(event `self.Col_SwitchFlashlight.OnComponentBeginOverlap`
  (params (OverlappedComponent :type "PrimitiveComponent Object Reference") (OtherActor :type "Actor Object Reference") (OtherComp :type "PrimitiveComponent Object Reference") (OtherBodyIndex :type Integer) (bFromSweep :type Boolean) (SweepResult :type "HitResult Structure (by ref)"))
  (`self.SwitchFlashlight`))

(fn `SimulateHandPhysics`
  (bind _handmodel_l (`self.HandModel_L`))
  (bind _handmodel_r (`self.HandModel_R`))
  (`|ExecutionSequence`
    (:`then_0`
      (`PhysicsConstraintComponent.SetConstrainedComponents` (`self.PhysicsConstraint`) (`self.LHandPosition`) "None" _handmodel_l "None")
      (`PrimitiveComponent.SetSimulatePhysics` _handmodel_l true)
      (`PrimitiveComponent.SetSimulatePhysics` _handmodel_l true))
    (:`then_1`
      (`PhysicsConstraintComponent.SetConstrainedComponents` (`self.PhysicsConstraint1`) (`self.RHandPosition`) "None" _handmodel_r "None")
      (`PrimitiveComponent.SetSimulatePhysics` _handmodel_r true))))

(fn `SwitchFlashlight`
  (if (`self.FlashlightOnHand?`)
    (`SceneComponent.K2_AttachToComponent` (`self.Flashlight`) (`self.Camera`) "None" "KeepRelative" "KeepRelative" "KeepRelative" true)
    (set `self.FlashlightOnHand?` true)
    (else
      (`SceneComponent.K2_AttachToComponent` (`self.Flashlight`) (`self.Camera`) "None" "KeepRelative" "KeepRelative" "KeepRelative" true)
      (set `self.FlashlightOnHand?` false)))
  (`SceneComponent.K2_AttachToComponent` (`self.Light`) (`self.Flashlight`) "None" "KeepRelative" "KeepRelative" "KeepRelative" true))

(fn `UserConstructionScript`)