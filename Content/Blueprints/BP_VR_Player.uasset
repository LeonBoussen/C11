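; VR player Blueprint that keeps its body in sync with the headset's tracked pose every tick.
; The capsule follows the headset: the actor moves by horizontal deltas and takes its yaw, while half-height is half the headset height.
; The camera receives only the remaining height, pitch and roll.
; HandOrigin is counter-offset by headset position and capsule half-height, with yaw set to actor yaw minus headset Z position.
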(event `self.ReceiveTick`
  (params (DeltaSeconds :type "Float (single-precision)"))
  (`self.CameraTransform`)
  (`self.CapsuleTransform`)
  (`self.HandOffset`))

(fn `CameraTransform`
  (bind (_devicerotation _deviceposition) (`HeadMountedDisplayFunctionLibrary.GetOrientationAndPosition`))
  (`SceneComponent.K2_SetRelativeLocationAndRotation` (`self.VRCamera`) (`KismetMathLibrary.MakeVector` 0.0 0.0 (- (.z _deviceposition) (`CapsuleComponent.CapsuleHalfHeight` (`self.CapsuleComponent`)))) (`KismetMathLibrary.MakeRotator` (.roll _devicerotation) (.pitch _devicerotation)) false false))

(fn `CapsuleTransform`
  (bind (_devicerotation _deviceposition) (`HeadMountedDisplayFunctionLibrary.GetOrientationAndPosition`))
  (bind (_devicerotation_2 _deviceposition_2) (`HeadMountedDisplayFunctionLibrary.GetOrientationAndPosition`))
  (bind (_storedlocation_x _storedlocation_y) (`KismetMathLibrary.BreakVector` (`self.StoredLocation`)))
  (`self.K2_AddActorLocalOffset` (`KismetMathLibrary.MakeVector` (- (.x _deviceposition_2) _storedlocation_x) (- (.y _deviceposition_2) _storedlocation_y)))
  (set `self.StoredLocation` (`KismetMathLibrary.MakeVector` (.x _deviceposition_2) (.y _deviceposition_2)))
  (`self.K2_SetActorRotation` (`KismetMathLibrary.MakeRotator` 0.0 0.0 (.yaw _devicerotation)))
  (`CapsuleComponent.SetCapsuleHalfHeight` (`self.CapsuleComponent`) (/ (.z _deviceposition) 2.0) true))

(fn `HandOffset`
  (bind (_returnvalue_roll _returnvalue_pitch _returnvalue_yaw) (`KismetMathLibrary.BreakRotator` (`self.K2_GetActorRotation`)))
  (bind (_devicerotation _deviceposition) (`HeadMountedDisplayFunctionLibrary.GetOrientationAndPosition`))
  (`SceneComponent.K2_SetWorldLocationAndRotation` (`self.handOrigin`) (- (`self.K2_GetActorLocation`) (`KismetMathLibrary.MakeVector` (.x _deviceposition) (.y _deviceposition) (`CapsuleComponent.CapsuleHalfHeight` (`self.CapsuleComponent`)))) (`KismetMathLibrary.MakeRotator` 0.0 0.0 (- _returnvalue_yaw (.z (`.DevicePosition` (`HeadMountedDisplayFunctionLibrary.GetOrientationAndPosition`))))) false false))

(fn `UserConstructionScript`)